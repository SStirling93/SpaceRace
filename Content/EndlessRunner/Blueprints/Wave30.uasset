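; Wave30 is an endless runner wave actor with rock and gem components that scrolls down the world Z axis and destroys itself far below the origin.
; Each Tick moves it down at a fixed speed, resets world rotation to zero and checks height for removal.
; RockRight and KingOfGem also get an upward offset, while they and RockKing spin in pitch.
; Zero-translation local transforms are also applied to RockKing and KingOfGem.
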(event `self.ReceiveTick`
  (params (DeltaSeconds :type "Float (single-precision)"))
  (bind _returnvalue (* 50.0 DeltaSeconds))
  (`|ExecutionSequence`
    (:`then_0`
      ;[1 1 1] Object movement
      (`|ExecutionSequence`
        (:`then_0`
          (`SceneComponent.K2_AddWorldOffset` (`self.rock right `) (`KismetMathLibrary.MakeVector` 0.0 0.0 _returnvalue) false)
          (`SceneComponent.K2_AddWorldOffset` (`self.king of gem`) (`KismetMathLibrary.MakeVector` 0.0 0.0 _returnvalue) false)
          (`SceneComponent.K2_AddWorldOffset` (`self.rock right `) (`KismetMathLibrary.MakeVector` 0.0 0.0 _returnvalue) false))
        (:`then_1`
          (`SceneComponent.K2_SetWorldRotation` (`KismetMathLibrary.MakeRot` (.pitch (struct)) (+ 0.0 (.yaw (struct))) (.roll (struct)))))
        (:`then_2`
          (`SceneComponent.K2_AddLocalRotation` (`self.rock king`) (`KismetMathLibrary.MakeRot` _returnvalue 0.0 0.0) false)
          (`SceneComponent.K2_AddLocalRotation` (`self.king of gem`) (`KismetMathLibrary.MakeRot` _returnvalue 0.0 0.0) false)
          (`SceneComponent.K2_AddLocalRotation` (`self.rock right `) (`KismetMathLibrary.MakeRot` _returnvalue 0.0 0.0) false))
        (:`then_3`
          (`SceneComponent.K2_AddLocalTransform` (`self.rock king`) (`KismetMathLibrary.MakeTransform` (`KismetMathLibrary.Conv_DoubleToVector` (* -10.0 0.0)) (struct) (1.0 1.0 1.0)) false))
        (:`then_4`
          (`SceneComponent.K2_AddLocalTransform` (`self.king of gem`) (`KismetMathLibrary.MakeTransform` (`KismetMathLibrary.Conv_DoubleToVector` (* -10.0 0.0)) (struct) (0.1 0.1 0.1)) false))))
    (:`then_1`
      ;[1 1 1] Destroy objects
      (`|ExecutionSequence`
        (:`then_0`
          (if (<= (.z (`SceneComponent.K2_GetComponentLocation`)) -20000.0)
            (`self.K2_DestroyActor`)))
        (:`then_1`
          (`SceneComponent.K2_AddWorldOffset` (`KismetMathLibrary.MakeVector` 0.0 0.0 (* DeltaSeconds -2000.0))))))))

(fn `UserConstructionScript`)