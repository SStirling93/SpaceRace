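; Rockswave32 is an endless-runner asteroid wave obstacle that travels down the Z axis and flags the player's ship on impact.
; Each Tick applies a frame-rate-scaled downward offset and destroys the actor once it falls below a Z threshold.
; Tick also runs movement, rotation and transform calls, mostly on Rock1, with zeroed offset and spin values.
; A hit on PaperSprite8 casts the other actor to ShipCharacter and sets its IsAsteroid flag.
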(event `self.ReceiveTick`
  (params (DeltaSeconds :type "Float (single-precision)"))
  (bind _returnvalue (* 0.0 DeltaSeconds))
  (`|ExecutionSequence`
    (:`then_0`
      ;[1 1 1] Object movement
      (`|ExecutionSequence`
        (:`then_0`
          (`SceneComponent.K2_AddWorldOffset` (`self.Rock1`) (`KismetMathLibrary.MakeVector` 0.0 0.0 _returnvalue) false))
        (:`then_1`
          (`SceneComponent.K2_SetWorldRotation` (`KismetMathLibrary.MakeRot` (.pitch (struct)) (+ 0.0 (.yaw (struct))) (.roll (struct)))))
        (:`then_2`
          (`SceneComponent.K2_AddLocalRotation` (`self.Rock1`) (`KismetMathLibrary.MakeRot` _returnvalue 0.0 0.0) false))
        (:`then_3`
          (`SceneComponent.K2_AddLocalTransform` (`self.Rock1`) (`KismetMathLibrary.MakeTransform` (`KismetMathLibrary.Conv_DoubleToVector` (* -10.0 0.0)) (struct) (1.5 1.5 1.5)) false))))
    (:`then_1`
      ;[1 1 1] Destroy objects
      (`|ExecutionSequence`
        (:`then_0`
          (if (<= (.z (`SceneComponent.K2_GetComponentLocation`)) -20000.0)
            (`self.K2_DestroyActor`)))
        (:`then_1`
          (`SceneComponent.K2_AddWorldOffset` (`KismetMathLibrary.MakeVector` 0.0 0.0 (* DeltaSeconds -1500.0))))))))

(event `self.PaperSprite8.OnComponentHit`
  (params (OtherActor :type "Actor Object Reference") (OtherComp :type "PrimitiveComponent Object Reference") (NormalImpulse :type "Object.Vector Structure") (Hit :type "EngineTypes.HitResult Structure (by ref)"))
  (bind _asship_character (cast `/Game/EndlessRunner/Blueprints/ShipCharacter` OtherActor))
  (set `/Game/EndlessRunner/Blueprints/ShipCharacter.IsAsteroid` true _asship_character))

(fn `UserConstructionScript`)