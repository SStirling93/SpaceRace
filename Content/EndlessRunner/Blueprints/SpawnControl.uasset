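; Spawner for the endless runner that places a random wave actor at its own location every five seconds.
; Tick accumulates time, then switches on a rounded-up random roll, with paired cases sharing each of fifteen wave classes (no Wave5).
; Waves spawn double-scale, slightly offset in Y, with the spawner's rotation; only Wave1 and Wave2 force spawning despite collision.
; A roll of 30 spawns nothing, and Lifetime is tracked without effect.
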(event `self.ReceiveTick`
  (params (DeltaSeconds :type "Float (single-precision)"))
  (bind _returnvalue (`KismetMathLibrary.MakeTransform` (`KismetMathLibrary.MakeVector` (.x (`SceneComponent.K2_GetComponentLocation`)) (+ (.y (`SceneComponent.K2_GetComponentLocation`)) 10.0) (.z (`SceneComponent.K2_GetComponentLocation`))) (`SceneComponent.K2_GetComponentRotation`) (2.0 2.0 2.0)))
  (bind _output_get (set `self.Counter` (+ DeltaSeconds (`self.Counter`))))
  (set `self.Lifetime` (+ DeltaSeconds (`self.Lifetime`)))
  (if (>= _output_get 5.0)
    (set `self.Counter` (- _output_get 5.0))
    (`KismetSystemLibrary.PrintString` "Hello")
    (switch `int` (`KismetMathLibrary.FCeil` (`KismetMathLibrary.RandomFloatInRange` 0.0 30.0))
      (:`0`
        (`|SpawnActorFromClass` "/Game/EndlessRunner/Blueprints/Wave1.Wave1_C" _returnvalue true :!label _label))
      (:`1`
        (goto _label))
      (:`2`
        (`|SpawnActorFromClass` "/Game/EndlessRunner/Blueprints/Wave2.Wave2_C" _returnvalue true :!label _label_2))
      (:`3`
        (goto _label_2))
      (:`4`
        (`|SpawnActorFromClass` "/Game/EndlessRunner/Blueprints/Wave3.Wave3_C" _returnvalue :!label _label_3))
      (:`5`
        (goto _label_3))
      (:`6`
        (`|SpawnActorFromClass` "/Game/EndlessRunner/Blueprints/Wave4.Wave4_C" _returnvalue :!label _label_4))
      (:`7`
        (goto _label_4))
      (:`8`
        (`|SpawnActorFromClass` "/Game/EndlessRunner/Blueprints/Wave6.Wave6_C" _returnvalue :!label _label_5))
      (:`9`
        (goto _label_5))
      (:`10`
        (`|SpawnActorFromClass` "/Game/EndlessRunner/Blueprints/Wave7.Wave7_C" _returnvalue :!label _label_6))
      (:`11`
        (goto _label_6))
      (:`12`
        (`|SpawnActorFromClass` "/Game/EndlessRunner/Blueprints/Wave8.Wave8_C" _returnvalue :!label _label_7))
      (:`13`
        (goto _label_7))
      (:`14`
        (`|SpawnActorFromClass` "/Game/EndlessRunner/Blueprints/Wave9.Wave9_C" _returnvalue :!label _label_8))
      (:`15`
        (goto _label_8))
      (:`16`
        (`|SpawnActorFromClass` "/Game/EndlessRunner/Blueprints/Wave10.Wave10_C" _returnvalue :!label _label_9))
      (:`17`
        (goto _label_9))
      (:`18`
        (`|SpawnActorFromClass` "/Game/EndlessRunner/Blueprints/Wave11.Wave11_C" _returnvalue :!label _label_10))
      (:`19`
        (goto _label_10))
      (:`20`
        (`|SpawnActorFromClass` "/Game/EndlessRunner/Blueprints/Wave12.Wave12_C" _returnvalue :!label _label_11))
      (:`21`
        (goto _label_11))
      (:`22`
        (`|SpawnActorFromClass` "/Game/EndlessRunner/Blueprints/Wave13.Wave13_C" _returnvalue :!label _label_12))
      (:`23`
        (goto _label_12))
      (:`24`
        (`|SpawnActorFromClass` "/Game/EndlessRunner/Blueprints/Wave14.Wave14_C" _returnvalue :!label _label_13))
      (:`25`
        (goto _label_13))
      (:`26`
        (`|SpawnActorFromClass` "/Game/EndlessRunner/Blueprints/Wave15.Wave15_C" _returnvalue :!label _label_14))
      (:`27`
        (goto _label_14))
      (:`28`
        (`|SpawnActorFromClass` "/Game/EndlessRunner/Blueprints/Wave16.Wave16_C" _returnvalue :!label _label_15))
      (:`29`
        (goto _label_15)))))

(event `self.ReceiveActorBeginOverlap`
  (params (OtherActor :type "Actor Object Reference")))

(event `self.ReceiveBeginPlay`)

(fn `UserConstructionScript`)