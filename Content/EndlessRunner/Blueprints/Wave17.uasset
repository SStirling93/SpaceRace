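; Wave17 is an endless runner wave actor holding an asteroid and a small ship that scroll down the world Z axis.
; Tick moves and spins the asteroid while nudging the ship with two opposing local transforms of unequal speed, all scaled by delta time.
; It also offsets the wave downward each frame and destroys the actor once it drops below a Z threshold.
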(event `self.ReceiveBeginPlay`
  ;[1 1 1] Object movement
)

(event `self.ReceiveActorBeginOverlap`
  (params (OtherActor :type "Actor Object Reference"))
  ;[1 1 1] Object movement
)

(event `self.ReceiveTick`
  (params (DeltaSeconds :type "Float (single-precision)"))
  (bind _returnvalue (* -500.0 DeltaSeconds))
  (`|ExecutionSequence`
    (:`then_0`
      ;[1 1 1] Object movement
      (`|ExecutionSequence`
        (:`then_0`
          (`SceneComponent.K2_AddWorldOffset` (`self.Asteriod`) (`KismetMathLibrary.MakeVector` 0.0 0.0 _returnvalue) false))
        (:`then_1`
          (`SceneComponent.K2_AddLocalTransform` (`self.Small ship`) (`KismetMathLibrary.MakeTransform` (`KismetMathLibrary.Conv_DoubleToVector` (* -10.0 DeltaSeconds)) (struct) (0.2 0.2 0.2)) false))
        (:`then_2`
          (`SceneComponent.K2_AddLocalRotation` (`self.Asteriod`) (`KismetMathLibrary.MakeRot` _returnvalue 0.0 0.0) false))
        (:`then_3`
          (`SceneComponent.K2_AddLocalTransform` (`self.Small ship`) (`KismetMathLibrary.MakeTransform` (`KismetMathLibrary.Conv_DoubleToVector` (* 50.0 DeltaSeconds)) (struct) (0.2 0.2 0.2)) false))))
    (:`then_1`
      ;[1 1 1] Destroy objects
      (`|ExecutionSequence`
        (:`then_0`
          (if (<= (.z (`SceneComponent.K2_GetComponentLocation`)) -5000.0)
            (`self.K2_DestroyActor`)))
        (:`then_1`
          (`SceneComponent.K2_AddWorldOffset` (`KismetMathLibrary.MakeVector` 0.0 0.0 (* DeltaSeconds -500.0))))))))

(fn `UserConstructionScript`)