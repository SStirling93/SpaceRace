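; BP_Laser is a laser projectile in the endless runner, built from a projectile movement component, a sphere and two Paper2D sprites.
; When it hits another BP_Laser, it strips that laser's sprites and hit component, then destroys itself.
; When projectile movement stops, it removes its own sprites and sphere through the same helper function, leaving the actor alive.
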(event `self.ReceiveBeginPlay`)

(event `self.ReceiveTick`
  (params (DeltaSeconds :type "Float (single-precision)")))

(event `self.ReceiveActorBeginOverlap`
  (params (OtherActor :type "Actor Object Reference")))

(event `self.ReceiveHit`
  (params (MyComp :type "PrimitiveComponent Object Reference") (Other :type "Actor Object Reference") (OtherComp :type "PrimitiveComponent Object Reference") (bSelfMoved :type Boolean) (HitLocation :type "Object.Vector Structure") (HitNormal :type "Object.Vector Structure") (NormalImpulse :type "Object.Vector Structure") (Hit :type "EngineTypes.HitResult Structure (by ref)"))
  (bind _asbp_laser (cast `/Game/EndlessRunner/Blueprints/BP_Laser` Other))
  (`self.Destroy component` _asbp_laser OtherComp)
  (`self.K2_DestroyActor`))

(event `self.ProjectileMovement.OnProjectileStop`
  (params (ImpactResult :type "EngineTypes.HitResult Structure (by ref)"))
  (`self.Destroy component` (`self.Sphere`)))

(fn `Destroy component`
  (params (component :type "ActorComponent Object Reference"))
  (`ActorComponent.K2_DestroyComponent` (`self.PaperSprite`))
  (`ActorComponent.K2_DestroyComponent` (`self.PaperSprite1`))
  (`ActorComponent.K2_DestroyComponent` component))

(fn `NewFunction_0`
  (params (NewParam :type "DestructibleComponent Class Reference")))

(fn `UserConstructionScript`)