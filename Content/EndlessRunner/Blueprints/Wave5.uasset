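; Wave5 is an endless runner wave actor that carries ships and an asteroid downward through the level.
; Tick shifts the whole actor along negative world Z at a frame-rate-scaled speed and destroys it once it falls past a lower Z limit.
; On top of that, the asteroid spins in pitch while the two leader ships drift in opposite local diagonal directions.
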(event `self.ReceiveActorBeginOverlap`
  (params (OtherActor :type "Actor Object Reference")))

(event `self.ReceiveBeginPlay`)

(event `self.ReceiveTick`
  (params (DeltaSeconds :type "Float (single-precision)"))
  (`|ExecutionSequence`
    (:`then_0`
      ;[1 1 1] Object movement
      (`|ExecutionSequence`
        (:`then_0`
          (`SceneComponent.K2_AddWorldOffset` (`self.Asteriod`) (0.0 0.0 0.0) false))
        (:`then_1`
          (`SceneComponent.K2_AddLocalTransform` (`self.Leader ship 2`) (`KismetMathLibrary.MakeTransform` (`KismetMathLibrary.Conv_DoubleToVector` (* -50.0 DeltaSeconds)) (struct) (0.2 0.2 0.2)) false))
        (:`then_2`
          (`SceneComponent.K2_AddLocalRotation` (`self.Asteriod`) (`KismetMathLibrary.MakeRot` (* -500.0 DeltaSeconds) 0.0 0.0) false))
        (:`then_3`
          (`SceneComponent.K2_AddLocalTransform` (`self.Group leader ship`) (`KismetMathLibrary.MakeTransform` (`KismetMathLibrary.Conv_DoubleToVector` (* 50.0 DeltaSeconds)) (struct) (0.2 0.2 0.2)) false))))
    (:`then_1`
      ;[1 1 1] Destroy objects
      (`|ExecutionSequence`
        (:`then_0`
          (if (<= (.z (`SceneComponent.K2_GetComponentLocation`)) -5000.0)
            (`self.K2_DestroyActor`)))
        (:`then_1`
          (`SceneComponent.K2_AddWorldOffset` (`KismetMathLibrary.MakeVector` 0.0 0.0 (* DeltaSeconds -500.0))))))))

(fn `UserConstructionScript`)