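; Boss2 is an endless runner actor with two boss components and an asteroid component that moves down through the level.
; On hit, either boss component triggers adding a Paper2D flipbook at a relative transform, likely an explosion effect, and a component is destroyed.
; Tick applies a constant downward Z offset and destroys the actor below a height limit.
; The other per-frame movement and rotation deltas are zeroed.
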(event `self.Boss.OnComponentHit`
  (params (OtherActor :type "Actor Object Reference") (OtherComp :type "PrimitiveComponent Object Reference") (NormalImpulse :type "Object.Vector Structure") (Hit :type "EngineTypes.HitResult Structure (by ref)"))
  (bind _returnvalue (`SceneComponent.GetRelativeTransform`))
  (`AddComponent|PaperFlipbookComponent_121` :`RelativeTransform` _returnvalue)
  (`ActorComponent.K2_DestroyComponent`))

(event `self.Boss 2.OnComponentHit`
  (params (OtherActor :type "Actor Object Reference") (OtherComp :type "PrimitiveComponent Object Reference") (NormalImpulse :type "Object.Vector Structure") (Hit :type "EngineTypes.HitResult Structure (by ref)"))
  (bind _returnvalue (`SceneComponent.GetRelativeTransform`))
  (`AddComponent|PaperFlipbookComponent_120` :`RelativeTransform` _returnvalue)
  (`ActorComponent.K2_DestroyComponent`))

(event `self.ReceiveTick`
  (params (DeltaSeconds :type "Float (single-precision)"))
  (bind _returnvalue (* 0.0 DeltaSeconds))
  (`|ExecutionSequence`
    (:`then_0`
      ;[1 1 1] Object movement
      (`|ExecutionSequence`
        (:`then_0`
          (`SceneComponent.K2_AddWorldOffset` (`self.Asteriod`) (`KismetMathLibrary.MakeVector` 0.0 0.0 _returnvalue) false)
          (`SceneComponent.K2_SetWorldRotation` (`KismetMathLibrary.MakeRot` (.pitch (`SceneComponent.K2_GetComponentRotation` (`self.Root`))) (+ 0.0 (.yaw (`SceneComponent.K2_GetComponentRotation` (`self.Root`)))) (.roll (`SceneComponent.K2_GetComponentRotation` (`self.Root`))))))
        (:`then_1`
          (`SceneComponent.K2_AddLocalTransform` (`self.Boss`) (`KismetMathLibrary.MakeTransform` (`KismetMathLibrary.Conv_DoubleToVector` (* 0.0 DeltaSeconds)) (struct) (0.2 0.2 0.2)) false))
        (:`then_2`
          (`SceneComponent.K2_AddLocalRotation` (`self.Asteriod`) (`KismetMathLibrary.MakeRot` _returnvalue 0.0 0.0) false))
        (:`then_3`
          (`SceneComponent.K2_AddLocalTransform` (`self.Boss 2`) (`KismetMathLibrary.MakeTransform` (`KismetMathLibrary.Conv_DoubleToVector` (* 0.0 DeltaSeconds)) (struct) (0.2 0.2 0.2)) false))))
    (:`then_1`
      ;[1 1 1] Destroy objects
      (`|ExecutionSequence`
        (:`then_0`
          (if (<= (.z (`SceneComponent.K2_GetComponentLocation`)) -5000.0)
            (`self.K2_DestroyActor`)))
        (:`then_1`
          (`SceneComponent.K2_AddWorldOffset` (`KismetMathLibrary.MakeVector` 0.0 0.0 (* DeltaSeconds -500.0))))))))

(fn `UserConstructionScript`)