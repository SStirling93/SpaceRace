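; Endless-runner obstacle wave actor with an asteroid and a small pirate that travel down world Z.
; Tick applies frame-scaled offsets and spins, and destroys the actor once the tracked Z position reaches a lower limit.
; A pirate hit on a ShipCharacter calls its Death, sets IsShip, adds a flipbook component and destroys a component.
; An asteroid hit starts a timed MoveComponentTo toward a fixed relative location.
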(event `self.Asteroid 1.OnComponentHit`
  (params (OtherActor :type "Actor Object Reference") (OtherComp :type "PrimitiveComponent Object Reference") (NormalImpulse :type "Object.Vector Structure") (Hit :type "EngineTypes.HitResult Structure (by ref)"))
  (`KismetSystemLibrary.MoveComponentTo` null (-50.0 -50.0 -50.0) (struct) false false 5.0))

(event `self.Small Pirate.OnComponentHit`
  (params (OtherActor :type "Actor Object Reference") (OtherComp :type "PrimitiveComponent Object Reference") (NormalImpulse :type "Object.Vector Structure") (Hit :type "EngineTypes.HitResult Structure (by ref)"))
  (bind _asship_character (cast `/Game/EndlessRunner/Blueprints/ShipCharacter` OtherActor))
  (`/Game/EndlessRunner/Blueprints/ShipCharacter.Death` _asship_character)
  (set `/Game/EndlessRunner/Blueprints/ShipCharacter.IsShip` true _asship_character)
  (bind _returnvalue (`SceneComponent.GetRelativeTransform`))
  (`AddComponent|Paper Flipbook Component_0` :`RelativeTransform` _returnvalue)
  (`ActorComponent.K2_DestroyComponent`))

(event `self.ReceiveTick`
  (params (DeltaSeconds :type "Float (single-precision)"))
  (bind _returnvalue (* -500.0 DeltaSeconds))
  (`|ExecutionSequence`
    (:`then_0`
      ;[1 1 1] Object movement
      (`|ExecutionSequence`
        (:`then_0`
          (`SceneComponent.K2_AddWorldOffset` (`self.Asteroid 1`) (`KismetMathLibrary.MakeVector` 0.0 0.0 _returnvalue) false))
        (:`then_1`
          (`SceneComponent.K2_SetWorldRotation` (`KismetMathLibrary.MakeRot` (.pitch (`SceneComponent.K2_GetComponentRotation` (`self.Root`))) (+ _returnvalue (.yaw (`SceneComponent.K2_GetComponentRotation` (`self.Root`)))) (.roll (`SceneComponent.K2_GetComponentRotation` (`self.Root`))))))
        (:`then_2`
          (`SceneComponent.K2_AddLocalRotation` (`self.Asteroid 1`) (`KismetMathLibrary.MakeRot` _returnvalue 0.0 0.0) false))))
    (:`then_1`
      ;[1 1 1] Destroy objects
      (`|ExecutionSequence`
        (:`then_0`
          (if (<= (.z (`SceneComponent.K2_GetComponentLocation`)) -5000.0)
            (`self.K2_DestroyActor`)))
        (:`then_1`
          (`SceneComponent.K2_AddWorldOffset` (`KismetMathLibrary.MakeVector` 0.0 0.0 (* DeltaSeconds -500.0))))))))

(event `self.ReceiveBeginPlay`)

(fn `UserConstructionScript`)