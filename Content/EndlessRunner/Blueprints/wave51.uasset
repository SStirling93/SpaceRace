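; Endless runner wave actor that moves steadily downward along world Z and destroys itself past a low height threshold.
; Every Tick, nested Sequences drift and pitch-spin the King component, reset a world rotation to zero, and apply two local transform offsets to the Right component.
; All logic is frame-driven, though only part of the Right offsets scales with delta time; the construction script is empty.
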(event `self.ReceiveBeginPlay`)

(event `self.ReceiveActorBeginOverlap`
  (params (OtherActor :type "Actor Object Reference")))

(event `self.ReceiveTick`
  (params (DeltaSeconds :type "Float (single-precision)"))
  (bind _returnvalue (* -40.0 DeltaSeconds))
  (`|ExecutionSequence`
    (:`then_0`
      ;[1 1 1] Object movement
      (`|ExecutionSequence`
        (:`then_0`
          (`SceneComponent.K2_AddWorldOffset` (`self.King`) (`KismetMathLibrary.MakeVector` 0.0 0.0 _returnvalue) false))
        (:`then_1`
          (`SceneComponent.K2_SetWorldRotation` (`KismetMathLibrary.MakeRot` (.pitch (struct)) (+ 0.0 (.yaw (struct))) (.roll (struct)))))
        (:`then_2`
          (`SceneComponent.K2_AddLocalRotation` (`self.King`) (`KismetMathLibrary.MakeRot` _returnvalue 0.0 0.0) false))
        (:`then_3`
          (`SceneComponent.K2_AddLocalTransform` (`self.right`) (`KismetMathLibrary.MakeTransform` (- (18.0 0.0 0.0) (* -0.3 DeltaSeconds)) (struct) (0.3 0.3 0.3)) false))
        (:`then_4`
          (`SceneComponent.K2_AddLocalTransform` (`self.right`) (`KismetMathLibrary.MakeTransform` (- (0.0 0.0 0.0) (* -0.3 DeltaSeconds)) (struct) (0.3 0.3 0.3)) false))))
    (:`then_1`
      ;[1 1 1] Destroy objects
      (`|ExecutionSequence`
        (:`then_0`
          (if (<= (.z (`SceneComponent.K2_GetComponentLocation`)) -5000.0)
            (`self.K2_DestroyActor`)))
        (:`then_1`
          (`SceneComponent.K2_AddWorldOffset` (`KismetMathLibrary.MakeVector` 0.0 0.0 (* DeltaSeconds -2000.0))))))))

(fn `UserConstructionScript`)