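; Wave18 is an Endless Runner Paper2D sprite object, likely an obstacle wave, that travels down the world Z axis.
; Each Tick it moves at a constant frame-rate-independent speed, holds world rotation at zero and destroys itself once far below the origin.
; The sprite's own offset and spin steps are zeroed out, and a scaling transform node is left unconnected.
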(event `ReceiveTick_Copy`
  (params (DeltaSeconds :type "Float (double-precision)" :default 0.0))
  (`|ExecutionSequence` :!label _label
    (:`then_0`
      ;[1 1 1] Object movement
      (`|ExecutionSequence`
        (:`then_0`
          (bind _returnvalue (* (stale `self.ReceiveTick` DeltaSeconds) 0.0))
          (`SceneComponent.K2_AddWorldOffset` (`self.PaperSprite`) (`KismetMathLibrary.MakeVector` 0.0 0.0 _returnvalue) false))
        (:`then_1`
          (`SceneComponent.K2_SetWorldRotation` (`KismetMathLibrary.MakeRot` (.pitch (struct)) (+ 0.0 (.yaw (struct))) (.roll (struct)))))
        (:`then_2`
          (`SceneComponent.K2_AddLocalRotation` (`self.PaperSprite`) (`KismetMathLibrary.MakeRot` _returnvalue 0.0 0.0) false))))
    (:`then_1`
      ;[1 1 1] Destroy objects
      (`|ExecutionSequence`
        (:`then_0`
          (if (<= (.z (`SceneComponent.K2_GetComponentLocation`)) -300000.0)
            (`self.K2_DestroyActor`)))
        (:`then_1`
          (`SceneComponent.K2_AddWorldOffset` (`KismetMathLibrary.MakeVector` 0.0 0.0 (* (stale `self.ReceiveTick` DeltaSeconds) -1500.0))))))))

(event `self.ReceiveTick`
  (params (DeltaSeconds :type "Float (single-precision)"))
  (goto _label))

(fn `UserConstructionScript`)