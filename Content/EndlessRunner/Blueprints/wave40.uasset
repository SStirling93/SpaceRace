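; Endless-runner wave actor built from Paper2D sprite pieces that descends along world Z and destroys itself once far below the level.
; Tick also zeroes world rotation, nudges and spins the DiamondKing piece, and applies per-frame local transforms to the left and right parts.
; Each piece has an identical, duplicated hit handler that adds a flipbook component using a relative transform, then calls DestroyComponent.
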(event `self.ReceiveTick`
  (params (DeltaSeconds :type "Float (single-precision)"))
  (bind _returnvalue (* 10.0 DeltaSeconds))
  (`|ExecutionSequence`
    (:`then_0`
      ;[1 1 1] Object movement
      (`|ExecutionSequence`
        (:`then_0`
          (`SceneComponent.K2_AddWorldOffset` (`self.diamond king`) (`KismetMathLibrary.MakeVector` 0.0 0.0 _returnvalue) false))
        (:`then_1`
          (`SceneComponent.K2_SetWorldRotation` (`KismetMathLibrary.MakeRot` (.pitch (struct)) (+ 0.0 (.yaw (struct))) (.roll (struct)))))
        (:`then_2`
          (`SceneComponent.K2_AddLocalRotation` (`self.diamond king`) (`KismetMathLibrary.MakeRot` _returnvalue 0.0 0.0) false))
        (:`then_3`
          (`SceneComponent.K2_AddLocalTransform` (`self.RightPart`) (`KismetMathLibrary.MakeTransform` (- (3.8 0.0 0.0) (* -2.0 DeltaSeconds)) (struct) (0.3 0.3 0.3)) false))
        (:`then_4`
          (`SceneComponent.K2_AddLocalTransform` (`self.Leftpart`) (`KismetMathLibrary.MakeTransform` (- (-3.8 0.0 0.0) (* -2.0 DeltaSeconds)) (struct) (0.3 0.3 0.3)) false))))
    (:`then_1`
      ;[1 1 1] Destroy objects
      (`|ExecutionSequence`
        (:`then_0`
          (if (<= (.z (`SceneComponent.K2_GetComponentLocation`)) -5000.0)
            (`self.K2_DestroyActor`)))
        (:`then_1`
          (`SceneComponent.K2_AddWorldOffset` (`KismetMathLibrary.MakeVector` 0.0 0.0 (* DeltaSeconds -500.0))))))))

(event `self.Leftpart.OnComponentHit`
  (params (OtherActor :type "Actor Object Reference") (OtherComp :type "PrimitiveComponent Object Reference") (NormalImpulse :type "Object.Vector Structure") (Hit :type "EngineTypes.HitResult Structure (by ref)"))
  (bind _returnvalue (`SceneComponent.GetRelativeTransform`))
  (`AddComponent|PaperFlipbookComponent_327` :`RelativeTransform` _returnvalue)
  (`ActorComponent.K2_DestroyComponent`))

(event `self.PaperSprite2.OnComponentHit`
  (params (OtherActor :type "Actor Object Reference") (OtherComp :type "PrimitiveComponent Object Reference") (NormalImpulse :type "Object.Vector Structure") (Hit :type "EngineTypes.HitResult Structure (by ref)"))
  (bind _returnvalue (`SceneComponent.GetRelativeTransform`))
  (`AddComponent|PaperFlipbookComponent_328` :`RelativeTransform` _returnvalue)
  (`ActorComponent.K2_DestroyComponent`))

(event `self.PaperSprite3.OnComponentHit`
  (params (OtherActor :type "Actor Object Reference") (OtherComp :type "PrimitiveComponent Object Reference") (NormalImpulse :type "Object.Vector Structure") (Hit :type "EngineTypes.HitResult Structure (by ref)"))
  (bind _returnvalue (`SceneComponent.GetRelativeTransform`))
  (`AddComponent|PaperFlipbookComponent_329` :`RelativeTransform` _returnvalue)
  (`ActorComponent.K2_DestroyComponent`))

(event `self.PaperSprite4.OnComponentHit`
  (params (OtherActor :type "Actor Object Reference") (OtherComp :type "PrimitiveComponent Object Reference") (NormalImpulse :type "Object.Vector Structure") (Hit :type "EngineTypes.HitResult Structure (by ref)"))
  (bind _returnvalue (`SceneComponent.GetRelativeTransform`))
  (`AddComponent|PaperFlipbookComponent_330` :`RelativeTransform` _returnvalue)
  (`ActorComponent.K2_DestroyComponent`))

(event `self.PaperSprite5.OnComponentHit`
  (params (OtherActor :type "Actor Object Reference") (OtherComp :type "PrimitiveComponent Object Reference") (NormalImpulse :type "Object.Vector Structure") (Hit :type "EngineTypes.HitResult Structure (by ref)"))
  (bind _returnvalue (`SceneComponent.GetRelativeTransform`))
  (`AddComponent|PaperFlipbookComponent_331` :`RelativeTransform` _returnvalue)
  (`ActorComponent.K2_DestroyComponent`))

(event `self.PaperSprite6.OnComponentHit`
  (params (OtherActor :type "Actor Object Reference") (OtherComp :type "PrimitiveComponent Object Reference") (NormalImpulse :type "Object.Vector Structure") (Hit :type "EngineTypes.HitResult Structure (by ref)"))
  (bind _returnvalue (`SceneComponent.GetRelativeTransform`))
  (`AddComponent|PaperFlipbookComponent_332` :`RelativeTransform` _returnvalue)
  (`ActorComponent.K2_DestroyComponent`))

(event `self.PaperSprite7.OnComponentHit`
  (params (OtherActor :type "Actor Object Reference") (OtherComp :type "PrimitiveComponent Object Reference") (NormalImpulse :type "Object.Vector Structure") (Hit :type "EngineTypes.HitResult Structure (by ref)"))
  (bind _returnvalue (`SceneComponent.GetRelativeTransform`))
  (`AddComponent|PaperFlipbookComponent_333` :`RelativeTransform` _returnvalue)
  (`ActorComponent.K2_DestroyComponent`))

(event `self.PaperSprite1.OnComponentHit`
  (params (OtherActor :type "Actor Object Reference") (OtherComp :type "PrimitiveComponent Object Reference") (NormalImpulse :type "Object.Vector Structure") (Hit :type "EngineTypes.HitResult Structure (by ref)"))
  (bind _returnvalue (`SceneComponent.GetRelativeTransform`))
  (`AddComponent|PaperFlipbookComponent_334` :`RelativeTransform` _returnvalue)
  (`ActorComponent.K2_DestroyComponent`))

(event `self.PaperSprite.OnComponentHit`
  (params (OtherActor :type "Actor Object Reference") (OtherComp :type "PrimitiveComponent Object Reference") (NormalImpulse :type "Object.Vector Structure") (Hit :type "EngineTypes.HitResult Structure (by ref)"))
  (bind _returnvalue (`SceneComponent.GetRelativeTransform`))
  (`AddComponent|PaperFlipbookComponent_335` :`RelativeTransform` _returnvalue)
  (`ActorComponent.K2_DestroyComponent`))

(event `self.RightPart.OnComponentHit`
  (params (OtherActor :type "Actor Object Reference") (OtherComp :type "PrimitiveComponent Object Reference") (NormalImpulse :type "Object.Vector Structure") (Hit :type "EngineTypes.HitResult Structure (by ref)"))
  (bind _returnvalue (`SceneComponent.GetRelativeTransform`))
  (`AddComponent|PaperFlipbookComponent_336` :`RelativeTransform` _returnvalue)
  (`ActorComponent.K2_DestroyComponent`))

(event `self.PaperSprite14.OnComponentHit`
  (params (OtherActor :type "Actor Object Reference") (OtherComp :type "PrimitiveComponent Object Reference") (NormalImpulse :type "Object.Vector Structure") (Hit :type "EngineTypes.HitResult Structure (by ref)"))
  (bind _returnvalue (`SceneComponent.GetRelativeTransform`))
  (`AddComponent|PaperFlipbookComponent_337` :`RelativeTransform` _returnvalue)
  (`ActorComponent.K2_DestroyComponent`))

(event `self.PaperSprite13.OnComponentHit`
  (params (OtherActor :type "Actor Object Reference") (OtherComp :type "PrimitiveComponent Object Reference") (NormalImpulse :type "Object.Vector Structure") (Hit :type "EngineTypes.HitResult Structure (by ref)"))
  (bind _returnvalue (`SceneComponent.GetRelativeTransform`))
  (`AddComponent|PaperFlipbookComponent_338` :`RelativeTransform` _returnvalue)
  (`ActorComponent.K2_DestroyComponent`))

(event `self.PaperSprite12.OnComponentHit`
  (params (OtherActor :type "Actor Object Reference") (OtherComp :type "PrimitiveComponent Object Reference") (NormalImpulse :type "Object.Vector Structure") (Hit :type "EngineTypes.HitResult Structure (by ref)"))
  (bind _returnvalue (`SceneComponent.GetRelativeTransform`))
  (`AddComponent|PaperFlipbookComponent_339` :`RelativeTransform` _returnvalue)
  (`ActorComponent.K2_DestroyComponent`))

(event `self.PaperSprite11.OnComponentHit`
  (params (OtherActor :type "Actor Object Reference") (OtherComp :type "PrimitiveComponent Object Reference") (NormalImpulse :type "Object.Vector Structure") (Hit :type "EngineTypes.HitResult Structure (by ref)"))
  (bind _returnvalue (`SceneComponent.GetRelativeTransform`))
  (`AddComponent|PaperFlipbookComponent_340` :`RelativeTransform` _returnvalue)
  (`ActorComponent.K2_DestroyComponent`))

(event `self.PaperSprite10.OnComponentHit`
  (params (OtherActor :type "Actor Object Reference") (OtherComp :type "PrimitiveComponent Object Reference") (NormalImpulse :type "Object.Vector Structure") (Hit :type "EngineTypes.HitResult Structure (by ref)"))
  (bind _returnvalue (`SceneComponent.GetRelativeTransform`))
  (`AddComponent|PaperFlipbookComponent_341` :`RelativeTransform` _returnvalue)
  (`ActorComponent.K2_DestroyComponent`))

(event `self.PaperSprite9.OnComponentHit`
  (params (OtherActor :type "Actor Object Reference") (OtherComp :type "PrimitiveComponent Object Reference") (NormalImpulse :type "Object.Vector Structure") (Hit :type "EngineTypes.HitResult Structure (by ref)"))
  (bind _returnvalue (`SceneComponent.GetRelativeTransform`))
  (`AddComponent|PaperFlipbookComponent_342` :`RelativeTransform` _returnvalue)
  (`ActorComponent.K2_DestroyComponent`))

(event `self.PaperSprite8.OnComponentHit`
  (params (OtherActor :type "Actor Object Reference") (OtherComp :type "PrimitiveComponent Object Reference") (NormalImpulse :type "Object.Vector Structure") (Hit :type "EngineTypes.HitResult Structure (by ref)"))
  (bind _returnvalue (`SceneComponent.GetRelativeTransform`))
  (`AddComponent|PaperFlipbookComponent_343` :`RelativeTransform` _returnvalue)
  (`ActorComponent.K2_DestroyComponent`))

(event `self.PaperSprite15.OnComponentHit`
  (params (OtherActor :type "Actor Object Reference") (OtherComp :type "PrimitiveComponent Object Reference") (NormalImpulse :type "Object.Vector Structure") (Hit :type "EngineTypes.HitResult Structure (by ref)"))
  (bind _returnvalue (`SceneComponent.GetRelativeTransform`))
  (`AddComponent|PaperFlipbookComponent_344` :`RelativeTransform` _returnvalue)
  (`ActorComponent.K2_DestroyComponent`))

(fn `UserConstructionScript`)