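; Scrolling Paper2D sprite layer piece for the endless runner, apparently one of a set of layer objects.
; Each Tick it moves down world Z at a constant, frame-rate-independent speed and destroys itself once it falls below a fixed height.
; The sprite movement and rotation nodes also run every frame, but their zero values leave them with no visible effect.
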(event `self.ReceiveTick`
  (params (DeltaSeconds :type "Float (single-precision)"))
  (bind _returnvalue (* 0.0 DeltaSeconds))
  (`|ExecutionSequence`
    (:`then_0`
      ;[1 1 1] Object movement
      (`|ExecutionSequence`
        (:`then_0`
          (`SceneComponent.K2_AddWorldOffset` (`self.PaperSprite`) (`KismetMathLibrary.MakeVector` 0.0 0.0 _returnvalue) false)
          (`SceneComponent.K2_SetWorldRotation` (`KismetMathLibrary.MakeRot` (.pitch (`SceneComponent.K2_GetComponentRotation` (`self.Root`))) (+ 0.0 (.yaw (`SceneComponent.K2_GetComponentRotation` (`self.Root`)))) (.roll (`SceneComponent.K2_GetComponentRotation` (`self.Root`))))))
        (:`then_2`
          (`SceneComponent.K2_AddLocalRotation` (`self.PaperSprite`) (`KismetMathLibrary.MakeRot` _returnvalue 0.0 0.0) false))))
    (:`then_1`
      ;[1 1 1] Destroy objects
      (`|ExecutionSequence`
        (:`then_0`
          (if (<= (.z (`SceneComponent.K2_GetComponentLocation`)) -20000.0)
            (`self.K2_DestroyActor`)))
        (:`then_1`
          (`SceneComponent.K2_AddWorldOffset` (`KismetMathLibrary.MakeVector` 0.0 0.0 (* DeltaSeconds -1500.0))))))))

(event `self.ReceiveBeginPlay`)

(event `self.ReceiveActorBeginOverlap`
  (params (OtherActor :type "Actor Object Reference")))

(fn `UserConstructionScript`)