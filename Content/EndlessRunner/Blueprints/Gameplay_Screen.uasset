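; Gameplay screen actor for an endless runner that populates itself with randomly placed obstacles through child actor components.
; Its construction script caches three top marker transforms and adds an enlarged asteroid, drawing location and rotation from separate random picks.
; A parallel pair of functions gathers seven top, side and corner markers for random ship spawns, but nothing here calls them.
; GetAttachTransform is an empty stub.
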(fn `GetAttachTransform`
  (returns (AttachTransform :type "Object.Transform Structure"))
  (return))

(fn `SetAsteroidSpawnPoints`
  (bind _returnvalue (`SceneComponent.GetRelativeTransform` (`self.TopLeft`)))
  (bind _returnvalue_2 (`SceneComponent.GetRelativeTransform` (`self.TopMiddle`)))
  (bind _returnvalue_3 (`SceneComponent.GetRelativeTransform` (`self.TopRight`)))
  (set `self.AsteroidSpawnPoints` (`|MakeArray` _returnvalue _returnvalue_2 _returnvalue_3)))

(fn `SetShipSpawnPoints`
  (bind _returnvalue (`SceneComponent.GetRelativeTransform` (`self.LeftTop`)))
  (bind _returnvalue_2 (`SceneComponent.GetRelativeTransform` (`self.LeftCorner`)))
  (bind _returnvalue_3 (`SceneComponent.GetRelativeTransform` (`self.TopLeft`)))
  (bind _returnvalue_4 (`SceneComponent.GetRelativeTransform` (`self.TopMiddle`)))
  (bind _returnvalue_5 (`SceneComponent.GetRelativeTransform` (`self.TopRight`)))
  (bind _returnvalue_6 (`SceneComponent.GetRelativeTransform` (`self.RightCorner`)))
  (bind _returnvalue_7 (`SceneComponent.GetRelativeTransform` (`self.RightTop`)))
  (set `self.ShipSpawnPoints` (`|MakeArray` _returnvalue _returnvalue_2 _returnvalue_3 _returnvalue_4 _returnvalue_5 _returnvalue_6 _returnvalue_7)))

(fn `SpawnAsteroid`
  (bind _asteroidspawnpoints (`self.AsteroidSpawnPoints`))
  (`AddComponent|Child Actor Component_0` :`RelativeTransform` (`KismetMathLibrary.MakeTransform` (.location (`KismetArrayLibrary.Array_Get` _asteroidspawnpoints (`KismetMathLibrary.RandomIntegerInRange` 0 (`KismetArrayLibrary.Array_LastIndex` _asteroidspawnpoints)))) (.rotation (`KismetArrayLibrary.Array_Get` _asteroidspawnpoints (`KismetMathLibrary.RandomIntegerInRange` 0 (`KismetArrayLibrary.Array_LastIndex` _asteroidspawnpoints)))) (5.0 5.0 5.0))))

(fn `SpawnShip`
  (bind _shipspawnpoints (`self.ShipSpawnPoints`))
  (`AddComponent|Child Actor Component_0` :`RelativeTransform` (`KismetArrayLibrary.Array_Get` _shipspawnpoints (`KismetMathLibrary.RandomIntegerInRange` 0 (`KismetArrayLibrary.Array_LastIndex` _shipspawnpoints)))))

(fn `UserConstructionScript`
  (`self.SetAsteroidSpawnPoints`)
  (`self.SpawnAsteroid`))