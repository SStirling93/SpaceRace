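; Wave16 is an endless-runner wave actor that holds SmallPolices movers and destroys itself once it drops below a Z threshold.
; A tick-style event, ReceiveTick_Copy, sequences movement and cleanup; nothing in this graph calls it, and the standard Tick is disabled.
; Most offsets and rotations evaluate to zero, leaving SmallPolices1's delta-time-based local transform as the only effective motion.
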(event `ReceiveTick_Copy`
  (params (DeltaSeconds :type "Float (double-precision)" :default 0.0))
  (bind _returnvalue (* -500.0 0.0))
  (`|ExecutionSequence`
    (:`then_0`
      ;[1 1 1] Object movement
      (`|ExecutionSequence`
        (:`then_0`
          (`SceneComponent.K2_AddWorldOffset` (`self.Small polices2`) (`KismetMathLibrary.MakeVector` 0.0 0.0 _returnvalue) false))
        (:`then_1`
          (`SceneComponent.K2_SetWorldRotation` (`KismetMathLibrary.MakeRot` (.pitch (struct)) (+ 0.0 (.yaw (struct))) (.roll (struct)))))
        (:`then_2`
          (`SceneComponent.K2_AddLocalRotation` (`self.Small polices2`) (`KismetMathLibrary.MakeRot` _returnvalue 0.0 0.0) false))
        (:`then_3`
          (`SceneComponent.K2_AddLocalTransform` (`self.Small polices1`) (`KismetMathLibrary.MakeTransform` (`KismetMathLibrary.Conv_DoubleToVector` (* 50.0 DeltaSeconds)) (struct) (0.2 0.2 0.2)) false))))
    (:`then_1`
      ;[1 1 1] Destroy objects
      (`|ExecutionSequence`
        (:`then_0`
          (if (<= (.z (`SceneComponent.K2_GetComponentLocation`)) -5000.0)
            (`self.K2_DestroyActor`)))
        (:`then_1`
          (`SceneComponent.K2_AddWorldOffset` (`KismetMathLibrary.MakeVector` 0.0)))))))

(event `self.ReceiveTick`
  (params (DeltaSeconds :type "Float (single-precision)")))

(fn `UserConstructionScript`)