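; Wave2 is an endless runner wave Blueprint containing ship and asteroid components that travels down the world Z axis.
; Tick applies a frame-rate-scaled downward offset and destroys the actor once the checked location falls below a low Z threshold.
; Hits on Ship1 or Ship2 add a flipbook component, then destroy a component.
; Asteroid movement and rotation nodes are left unconnected and never run.
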(event `self.Ship 2.OnComponentHit`
  (params (OtherActor :type "Actor Object Reference") (OtherComp :type "PrimitiveComponent Object Reference") (NormalImpulse :type "Object.Vector Structure") (Hit :type "EngineTypes.HitResult Structure (by ref)"))
  (bind _returnvalue (`SceneComponent.GetRelativeTransform`))
  (`AddComponent|PaperFlipbookComponent_11` :`RelativeTransform` _returnvalue)
  (`ActorComponent.K2_DestroyComponent`))

(event `self.Ship 1.OnComponentHit`
  (params (OtherActor :type "Actor Object Reference") (OtherComp :type "PrimitiveComponent Object Reference") (NormalImpulse :type "Object.Vector Structure") (Hit :type "EngineTypes.HitResult Structure (by ref)"))
  (bind _returnvalue (`SceneComponent.GetRelativeTransform`))
  (`AddComponent|Paper Flipbook Component_38` :`RelativeTransform` _returnvalue)
  (`ActorComponent.K2_DestroyComponent`))

(event `self.ReceiveBeginPlay`)

(event `self.ReceiveActorBeginOverlap`
  (params (OtherActor :type "Actor Object Reference")))

(event `self.ReceiveTick`
  (params (DeltaSeconds :type "Float (single-precision)"))
  (`|ExecutionSequence`
    (:`then_1`
      ;[1 1 1] Destroy objects
      (`|ExecutionSequence`
        (:`then_0`
          (if (<= (.z (`SceneComponent.K2_GetComponentLocation`)) -20000.0)
            (`self.K2_DestroyActor`)))
        (:`then_1`
          (`SceneComponent.K2_AddWorldOffset` (`KismetMathLibrary.MakeVector` 0.0 0.0 (* DeltaSeconds -3000.0))))))))

(fn `UserConstructionScript`)