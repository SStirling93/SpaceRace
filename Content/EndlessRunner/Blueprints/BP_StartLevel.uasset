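; BP_StartLevel is a level segment for an endless runner that scatters coins and chains in the next segment.
; Its construction script adds child actors, presumably coins, at random points inside the CoinArea box.
; When the ShipCharacter overlaps EndTrigger, it asks RunGameMode to add a level, then destroys itself after a short delay.
; GetAttachTransform exposes the AttachPoint world transform, apparently for placing the following segment.
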(event `self.EndTrigger.OnComponentBeginOverlap`
  (params (OtherActor :type "Actor Object Reference") (OtherComp :type "PrimitiveComponent Object Reference") (OtherBodyIndex :type Integer) (bFromSweep :type Boolean) (SweepResult :type "EngineTypes.HitResult Structure (by ref)"))
  (cast `/Game/EndlessRunner/Blueprints/ShipCharacter` OtherActor)
  (bind _asrun_game_mode (cast `/Game/EndlessRunner/Blueprints/RunGameMode` (`GameplayStatics.GetGameMode`)))
  (`/Game/EndlessRunner/Blueprints/RunGameMode.AddLevel` _asrun_game_mode)
  (`KismetSystemLibrary.Delay` 2.0)
  (`self.K2_DestroyActor`))

(fn `GetAttachTransform`
  (returns (AttachTransform :type "Object.Transform Structure"))
  (return (`SceneComponent.K2_GetComponentToWorld` (`self.AttachPoint`))))

(fn `SpawnCoins`
  (bind _coinarea (`self.CoinArea`))
  (for _ (range 11)
    (`AddComponent|Child Actor Component_0` :`RelativeTransform` (`KismetMathLibrary.Conv_VectorToTransform` (`KismetMathLibrary.RandomPointInBoundingBox` (`SceneComponent.RelativeLocation` _coinarea) (`BoxComponent.BoxExtent` _coinarea))))))

(fn `UserConstructionScript`
  (`self.SpawnCoins`))