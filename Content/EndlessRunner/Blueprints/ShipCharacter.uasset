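; Player ship character for a Paper2D endless runner, moving on the X and Z axes and replicating its sprite.
; Touch or Shoot input spawns a BP_Laser at an offset from the ship.
; A capsule hit stops the ship and plays an explosion, then after a delay Death destroys the actor and restarts the level.
; Score, coin gauge and level milestone logic are unfinished stubs, partly disconnected.
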(event `ReceiveBeginPlay_Copy_1`
  (set `self.High Score` (+ (`self.Score`) 1))
  (cast `HUD` (`PlayerController.GetHUD` (`GameplayStatics.GetPlayerController` 0))
    (:`then`
      _)
    (:`CastFailed`
      _))
  (set `self.High Score` (`self.Score`)))

(event `self.ReceiveBeginPlay`
  (`ActorComponent.SetIsReplicated` (`self.Sprite`) true))

(event `InputAxis|MoveXAxis`
  (params (AxisValue :type "Float (single-precision)"))
  ;[1 1 1] Handle movement
  (`self.AddMovementInput` (1.0 0.0 0.0) AxisValue))

(event `InputAxis|MoveZAxis`
  (params (AxisValue :type "Float (single-precision)"))
  ;[1 1 1] Handle movement
  (`self.AddMovementInput` (0.0 0.0 1.0) AxisValue))

(event `self.CapsuleComponent.OnComponentHit`
  (params (OtherActor :type "Actor Object Reference") (OtherComp :type "PrimitiveComponent Object Reference") (NormalImpulse :type "Object.Vector Structure") (Hit :type "EngineTypes.HitResult Structure (by ref)"))
  ;[1 1 1] Death of player ship
  (`AddComponent|Paper Flipbook Component_0`)
  (`MovementComponent.StopMovementImmediately`)
  (`self.DisableInput` null)
  (`GameplayStatics.PlaySoundAtLocation` "/Game/EndlessRunner/Sound/Explosion01.Explosion01")
  (`ActorComponent.K2_DestroyComponent`)
  (`ActorComponent.K2_DestroyComponent`)
  (`KismetSystemLibrary.Delay` 1.5)
  (`self.Death`))

(event `Death`
  (bind _returnvalue (`self.K2_GetActorLocation`))
  ;[1 1 1] Death Function
  (`self.DisableInput` null)
  (`CharacterMovementComponent.DisableMovement`)
  (`GameplayStatics.SpawnEmitterAtLocation` null _returnvalue)
  (`GameplayStatics.PlaySoundAtLocation` "/Game/EndlessRunner/Sound/Explosion01.Explosion01" _returnvalue)
  (`self.K2_DestroyActor`)
  (`KismetSystemLibrary.ExecuteConsoleCommand` "RestartLevel"))

(event `InputTouch`
  (params (Location :type "Object.Vector Structure" :default (0.0 0.0 0.0)) (FingerIndex :type "InputCoreTypes.ETouchIndex Enum"))
  (bind _returnvalue (`self.GetControlRotation`))
  (:`Pressed`
    (`|SpawnActorFromClass` "/Game/EndlessRunner/Blueprints/BP_Laser.BP_Laser_C" (`KismetMathLibrary.MakeTransform` (- (`self.K2_GetActorLocation`) (- (`KismetMathLibrary.GetUpVector` _returnvalue) 200.0)) _returnvalue) true :!label _label)))

(event `InputAction|Shoot`
  (:`Pressed`
    (goto _label)))

(event `ReceiveBeginPlay_Copy`
  ;[1 1 1] Coin gague on hud
  (bind _returnvalue (`|CreateWidget` "/Game/EndlessRunner/UMG/RunHUD.RunHUD_C"))
  (set `/Game/EndlessRunner/UMG/RunHUD.Coin gauge` null _returnvalue))

(fn `AddCoin`
  (set `self.High Score` 0))

(fn `NewFunction_0`)

(fn `NewFunction_1`
  (params (MinimumGems :type "Float (double-precision)") (`Current Gems` :type "Float (double-precision)")))

(fn `OnRep_High Score`)

(fn `UserConstructionScript`)